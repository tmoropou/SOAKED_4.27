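; BP_SniperSquirt is a pickup water sniper soaker that the player equips and fires.
; Interaction attaches it to the first-person mesh's pistol socket and registers it as the equipped weapon on the player.
; Fire, gated by WaterLevel, traces from the camera to find the aim point, then launches a projectile from the muzzle toward it with a squirt effect.
; Each shot drains water, and Unequip delegates to UnequipWeapon.
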(event `/Game/Interactables/Soakers/BPI_Weapon.Fire`
  (bind _returnvalue (`SceneComponent.GetSocketLocation` (`self.Mesh`) "MuzzleFlash"))
  (bind _firstpersoncamera (`FirstPersonCharacterBase.FirstPersonCamera` (`self.PlayerCharRef`)))
  (bind _returnvalue_2 (`SceneComponent.K2_GetComponentLocation` _firstpersoncamera))
  ;[1 1 1] Fire
  (if (> (`self.WaterLevel`) 0)
    (`GameplayStatics.SpawnEmitterAttached` "/Game/Particles/P_WaterSquirt.P_WaterSquirt" (`self.Mesh`) "MuzzleFlash")
    (bind _outhit (`KismetSystemLibrary.LineTraceSingle` :`Start` _returnvalue_2 :`End` (+ _returnvalue_2 (* (`SceneComponent.GetForwardVector` _firstpersoncamera) 100000.0)) :`TraceChannel` "TraceTypeQuery1" :`DrawDebugType` "ForOneFrame"))
    (`|SpawnActorFromClass` "/Game/Interactables/Soakers/Projectiles/SniperProjectile.SniperProjectile_C" (`KismetMathLibrary.MakeTransform` _returnvalue (`KismetMathLibrary.FindLookAtRotation` _returnvalue (`.Location` (`GameplayStatics.BreakHitResult` _outhit)))) "Undefined" "OverrideRootScale" null null)
    (set `self.WaterLevel` (- (`self.WaterLevel`) 5))))

(event `/Game/Interactables/BPI_Interact.Interaction`
  (params (Instigator :type "/Game/FirstPersonBP/Blueprints/FirstPersonCharacter Object Reference"))
  (`PrimitiveComponent.SetRenderCustomDepth` (`self.Mesh`) false)
  (set `/Game/FirstPersonBP/Blueprints/FirstPersonCharacter.gunEquipped` true (`self.PlayerCharRef`))
  (`self.K2_AttachToComponent` self (`/Game/FirstPersonBP/Blueprints/FirstPersonCharacter.Mesh1P` (`self.PlayerCharRef`)) "PistolSocket" "SnapToTarget" "SnapToTarget" "KeepRelative" true)
  (set `/Game/FirstPersonBP/Blueprints/FirstPersonCharacter.ItemAttached` self (`self.PlayerCharRef`))
  (set `/Game/FirstPersonBP/Blueprints/FirstPersonCharacter.WeaponAttached` "NewEnumerator4" (`self.PlayerCharRef`)))

(event `/Game/Interactables/Soakers/BPI_Weapon.Unequip`
  ;[1 1 1] Unequip Weapon
  (`self.UnequipWeapon`))

(fn `GetWaterLevel`
  (returns (WaterLevel :type Integer))
  (return (`self.WaterLevel`)))

(fn `UserConstructionScript`
  (`parent.UserConstructionScript`))