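; Interactable soaker weapon, apparently a base for main weapons, that the first-person player can highlight and unequip.
; Its overlap area toggles a custom-depth highlight and HUD prompt, registers itself on the player, and on exit cancels the hold-key timer and bar.
; Unequipping hides the player's attached item, stores it as ItemEquipped and clears the gun state.
; GetWaterLevel is a stub returning zero.
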(event `self.ReceiveBeginPlay`
  (bind _asfirst_person_character (cast `/Game/FirstPersonBP/Blueprints/FirstPersonCharacter` (`GameplayStatics.GetPlayerCharacter` 0)))
  (set `self.PlayerCharRef` _asfirst_person_character))

(event `self.InteractableArea.OnComponentBeginOverlap`
  (params (OverlappedComponent :type "PrimitiveComponent Object Reference") (OtherActor :type "Actor Object Reference") (OtherComp :type "PrimitiveComponent Object Reference") (OtherBodyIndex :type Integer) (bFromSweep :type Boolean) (SweepResult :type "HitResult Structure (by ref)"))
  (bind _playercharref (`self.PlayerCharRef`))
  (cast `/Game/FirstPersonBP/Blueprints/FirstPersonCharacter` OtherActor)
  (`PrimitiveComponent.SetRenderCustomDepth` (`self.Mesh`) true)
  (set `/Game/FirstPersonBP/Blueprints/FirstPersonCharacter.HighlightedInteractable` self _playercharref)
  (`/Game/FirstPersonBP/Widgets/MainHUD.ShowInteractionText` (cast `/Game/FirstPersonBP/Widgets/MainHUD` (`FirstPersonCharacterBase.MainHudRef` _playercharref) :!pure true))
  (set `/Game/FirstPersonBP/Blueprints/FirstPersonCharacter.OverlappingActor?` true (`self.PlayerCharRef`)))

(event `self.InteractableArea.OnComponentEndOverlap`
  (params (OverlappedComponent :type "PrimitiveComponent Object Reference") (OtherActor :type "Actor Object Reference") (OtherComp :type "PrimitiveComponent Object Reference") (OtherBodyIndex :type Integer))
  (bind _playercharref (`self.PlayerCharRef`))
  (cast `/Game/FirstPersonBP/Blueprints/FirstPersonCharacter` OtherActor)
  (`PrimitiveComponent.SetRenderCustomDepth` (`self.Mesh`) false)
  (`/Game/FirstPersonBP/Widgets/MainHUD.HideInteractionText` (cast `/Game/FirstPersonBP/Widgets/MainHUD` (`FirstPersonCharacterBase.MainHudRef` (`self.PlayerCharRef`)) :!pure true))
  (set `/Game/FirstPersonBP/Blueprints/FirstPersonCharacter.OverlappingActor?` false (`self.PlayerCharRef`))
  (`KismetSystemLibrary.K2_ClearTimer` _playercharref "IncrementHoldKeyValue")
  (`/Game/FirstPersonBP/Widgets/MainHUD.HideKeyHoldBar` (cast `/Game/FirstPersonBP/Widgets/MainHUD` (`FirstPersonCharacterBase.MainHudRef` _playercharref) :!pure true)))

(event `/Game/Interactables/Soakers/BPI_Weapon.Unequip`
  (`self.UnequipWeapon`))

(fn `GetWaterLevel`
  (returns (WaterLevel :type Integer))
  (return 0))

(fn `SetHighlight`
  (params (`Highlight?` :type Boolean))
  (`PrimitiveComponent.SetRenderCustomDepth` (`self.Mesh`) `Highlight?`))

(fn `UnequipWeapon`
  (bind _playercharref (`self.PlayerCharRef`))
  (bind _itemattached (`/Game/FirstPersonBP/Blueprints/FirstPersonCharacter.ItemAttached` (`self.PlayerCharRef`)))
  (`/Engine/EditorBlueprintResources/StandardMacros.IsValid` _itemattached
    (:`Is Valid`
      (`self.SetActorHiddenInGame` _itemattached true)
      (set `/Game/FirstPersonBP/Blueprints/FirstPersonCharacter.ItemEquipped` _itemattached _playercharref)
      (set `/Game/FirstPersonBP/Blueprints/FirstPersonCharacter.ItemAttached` null _playercharref)
      (set `/Game/FirstPersonBP/Blueprints/FirstPersonCharacter.WeaponAttached` "NewEnumerator2" _playercharref)
      (set `/Game/FirstPersonBP/Blueprints/FirstPersonCharacter.gunEquipped` false _playercharref))))

(fn `UserConstructionScript`)