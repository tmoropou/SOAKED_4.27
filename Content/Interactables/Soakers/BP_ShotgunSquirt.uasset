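; Shotgun-style water soaker weapon that fires a burst of water projectiles while it has water and is off cooldown.
; Fire traces from the player's first-person camera to find the aim point, with a one-frame debug line left on.
; SpawnProjectile launches four projectiles from the muzzle toward that point in a cross, offset in yaw and pitch by ShotgunSpread.
; Each shot plays a squirt emitter, drains WaterLevel and blocks firing for ReloadTime.
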(event `/Game/Interactables/Soakers/BPI_Weapon.Fire`
  (bind _firstpersoncamera (`FirstPersonCharacterBase.FirstPersonCamera` (`self.PlayerCharRef`)))
  (bind _returnvalue (`SceneComponent.K2_GetComponentLocation` _firstpersoncamera))
  ;[1 1 1] Fire
  (if (and (> (`self.WaterLevel`) 0) (not (`self.bCoolDown`)))
    (`GameplayStatics.SpawnEmitterAttached` "/Game/Particles/P_WaterSquirt.P_WaterSquirt" (`self.Mesh`) "MuzzleFlash")
    (bind _outhit (`KismetSystemLibrary.LineTraceSingle` :`Start` _returnvalue :`End` (+ _returnvalue (* (`SceneComponent.GetForwardVector` _firstpersoncamera) 100000.0)) :`TraceChannel` "TraceTypeQuery1" :`DrawDebugType` "ForOneFrame"))
    (bind (_bblockinghit _binitialoverlap _time _distance _location _impactpoint _normal _impactnormal _physmat _hitactor _hitcomponent _hitbonename _hititem _elementindex _faceindex _tracestart _traceend) (`GameplayStatics.BreakHitResult` _outhit))
    (if _bblockinghit
      (`self.SpawnProjectile` _impactpoint)
      (else
        (`self.SpawnProjectile` _traceend)))
    (set `self.WaterLevel` (- (`self.WaterLevel`) 20))
    (set `self.bCoolDown` true)
    (`KismetSystemLibrary.Delay` (`self.ReloadTime`))
    (set `self.bCoolDown` false)))

(event `/Game/Interactables/Soakers/BPI_Weapon.StopFiring`
  (`KismetSystemLibrary.K2_PauseTimer` null "StartFiring"))

(event `/Game/Interactables/Soakers/BPI_Weapon.Unequip`
  ;[1 1 1] Unequip Weapon
  (`self.UnequipWeapon`))

(fn `GetWaterLevel`
  (returns (WaterLevel :type Integer))
  (return (`self.WaterLevel`)))

(fn `SpawnProjectile`
  (params (`End Location` :type "Vector Structure"))
  (bind _returnvalue (`SceneComponent.GetSocketLocation` (`self.Mesh`) "MuzzleFlash"))
  (bind _returnvalue_2 (`SceneComponent.GetSocketLocation` (`self.Mesh`) "MuzzleFlash"))
  (bind _returnvalue_3 (`SceneComponent.GetSocketLocation` (`self.Mesh`) "MuzzleFlash"))
  (bind _returnvalue_4 (`SceneComponent.GetSocketLocation` (`self.Mesh`) "MuzzleFlash"))
  (bind (_returnvalue_roll _returnvalue_pitch _returnvalue_yaw) (`KismetMathLibrary.BreakRotator` (`KismetMathLibrary.FindLookAtRotation` _returnvalue (`local.End Location`))))
  (bind (_returnvalue_roll_2 _returnvalue_pitch_2 _returnvalue_yaw_2) (`KismetMathLibrary.BreakRotator` (`KismetMathLibrary.FindLookAtRotation` _returnvalue_2 (`local.End Location`))))
  (bind (_returnvalue_roll_3 _returnvalue_pitch_3 _returnvalue_yaw_3) (`KismetMathLibrary.BreakRotator` (`KismetMathLibrary.FindLookAtRotation` _returnvalue_3 (`local.End Location`))))
  (bind (_returnvalue_roll_4 _returnvalue_pitch_4 _returnvalue_yaw_4) (`KismetMathLibrary.BreakRotator` (`KismetMathLibrary.FindLookAtRotation` _returnvalue_4 (`local.End Location`))))
  (`|ExecutionSequence`
    (:`then_0`
      (`|SpawnActorFromClass` "/Game/Interactables/Soakers/Projectiles/WaterProjectile.WaterProjectile_C" (`KismetMathLibrary.MakeTransform` _returnvalue_2 (`KismetMathLibrary.MakeRotator` _returnvalue_roll_2 _returnvalue_pitch_2 (+ _returnvalue_yaw_2 (`self.ShotgunSpread`)))) "Undefined" "OverrideRootScale" null null))
    (:`then_1`
      (`|SpawnActorFromClass` "/Game/Interactables/Soakers/Projectiles/WaterProjectile.WaterProjectile_C" (`KismetMathLibrary.MakeTransform` _returnvalue_3 (`KismetMathLibrary.MakeRotator` _returnvalue_roll_3 _returnvalue_pitch_3 (- _returnvalue_yaw_3 (`self.ShotgunSpread`)))) "Undefined" "OverrideRootScale" null null))
    (:`then_2`
      (`|SpawnActorFromClass` "/Game/Interactables/Soakers/Projectiles/WaterProjectile.WaterProjectile_C" (`KismetMathLibrary.MakeTransform` _returnvalue_4 (`KismetMathLibrary.MakeRotator` _returnvalue_roll_4 (+ _returnvalue_pitch_4 (`self.ShotgunSpread`)) _returnvalue_yaw_4)) "Undefined" "OverrideRootScale" null null))
    (:`then_3`
      (`|SpawnActorFromClass` "/Game/Interactables/Soakers/Projectiles/WaterProjectile.WaterProjectile_C" (`KismetMathLibrary.MakeTransform` _returnvalue (`KismetMathLibrary.MakeRotator` _returnvalue_roll (- _returnvalue_pitch (`self.ShotgunSpread`)) _returnvalue_yaw)) "Undefined" "OverrideRootScale" null null)
      (return))))

(fn `UserConstructionScript`
  (`parent.UserConstructionScript`))