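; BP_AssaultSquirt is an automatic water gun that fires WaterProjectile actors while its WaterLevel lasts.
; Fire shoots immediately and starts a looping timer on StartFiring, which StopFiring pauses by name.
; Each shot plays a muzzle emitter and traces from the player's camera, aiming the muzzle-spawned projectile at the impact point or trace end.
; Water drains only when the trace hits; Unequip calls UnequipWeapon.
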(event `/Game/Interactables/Soakers/BPI_Weapon.Fire`
  ;[1 1 1] Fire
  (`self.StartFiring`)
  (`KismetSystemLibrary.K2_SetTimerDelegate` (delegate `StartFiring`) 0.2 true))

(event `StartFiring`
  (bind _returnvalue (`SceneComponent.GetSocketLocation` (`self.Mesh_Skel`) "MuzzleFlash"))
  (bind _returnvalue_2 (`SceneComponent.GetSocketLocation` (`self.Mesh_Skel`) "MuzzleFlash"))
  (bind _firstpersoncamera (`FirstPersonCharacterBase.FirstPersonCamera` (`self.PlayerCharRef`)))
  (bind _returnvalue_3 (`SceneComponent.K2_GetComponentLocation` _firstpersoncamera))
  ;[1 1 1] Fire
  (if (> (`self.WaterLevel`) 0)
    (`GameplayStatics.SpawnEmitterAttached` "/Game/Particles/P_WaterSquirt.P_WaterSquirt" (`self.Mesh_Skel`) "MuzzleFlash")
    (bind _outhit (`KismetSystemLibrary.LineTraceSingle` _returnvalue_3 (+ _returnvalue_3 (* (`SceneComponent.GetForwardVector` _firstpersoncamera) 100000.0)) "TraceTypeQuery1"))
    (bind (_bblockinghit _binitialoverlap _time _distance _location _impactpoint _normal _impactnormal _physmat _hitactor _hitcomponent _hitbonename _hititem _elementindex _faceindex _tracestart _traceend) (`GameplayStatics.BreakHitResult` _outhit))
    (if _bblockinghit
      (`|SpawnActorFromClass` "/Game/Interactables/Soakers/Projectiles/WaterProjectile.WaterProjectile_C" (`KismetMathLibrary.MakeTransform` _returnvalue_2 (`KismetMathLibrary.FindLookAtRotation` _returnvalue_2 _impactpoint)) "Undefined" "OverrideRootScale" null null)
      (set `self.WaterLevel` (- (`self.WaterLevel`) 2))
      (else
        (`|SpawnActorFromClass` "/Game/Interactables/Soakers/Projectiles/WaterProjectile.WaterProjectile_C" (`KismetMathLibrary.MakeTransform` _returnvalue (`KismetMathLibrary.FindLookAtRotation` _returnvalue _traceend)) "Undefined" "OverrideRootScale" null null)))))

(event `/Game/Interactables/Soakers/BPI_Weapon.StopFiring`
  (`KismetSystemLibrary.K2_PauseTimer` null "StartFiring"))

(event `/Game/Interactables/Soakers/BPI_Weapon.Unequip`
  ;[1 1 1] Unequip Weapon
  (`self.UnequipWeapon`))

(fn `UserConstructionScript`
  (`parent.UserConstructionScript`))