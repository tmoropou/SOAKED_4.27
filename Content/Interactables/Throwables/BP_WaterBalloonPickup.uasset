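; BP_WaterBalloonPickup is an interactable water balloon pickup that the player collects into their inventory.
; On Interaction, it checks HasSpace and, if that passes, calls PickupItem.
; PickupItem destroys the world actor, then adds BP_WaterBalloonPickup to the ItemInventory on PlayerCharRef.
; BeginPlay, overlap and Tick are unused.
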(event `/Game/Interactables/BPI_Interact.Interaction`
  (params (Instigator :type "/Game/FirstPersonBP/Blueprints/FirstPersonCharacter Object Reference") (Interactable :type "/Game/Interactables/BaseInteractable Object Reference"))
  (if (`self.HasSpace`)
    (`self.PickupItem`)))

(fn `PickupItem`
  (`self.K2_DestroyActor`)
  (`KismetArrayLibrary.Array_Add` (`/Game/FirstPersonBP/Blueprints/FirstPersonCharacter.ItemInventory` (`self.PlayerCharRef`)) "BP_WaterBalloonPickup_C"))

(fn `UserConstructionScript`
  (`parent.UserConstructionScript`))