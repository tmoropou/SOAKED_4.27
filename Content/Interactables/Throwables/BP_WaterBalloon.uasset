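; BP_WaterBalloon is a thrown water balloon projectile that bursts when it hits something.
; On BeginPlay it applies its Velocity to ProjectileMovement, tints the mesh through a dynamic material using the first entry of the player's WaterBalloonColor, and ignores the player when moving.
; On hit it hides the balloon and activates the WaterBurst effect, then destroys itself once that effect finishes.
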(event `self.ReceiveBeginPlay`
  (bind _asfirst_person_character (cast `/Game/FirstPersonBP/Blueprints/FirstPersonCharacter` (`GameplayStatics.GetPlayerCharacter` 0)))
  (set `self.PlayerRef` _asfirst_person_character)
  (set `MovementComponent.Velocity` (`self.Velocity`) (`self.ProjectileMovement`))
  (bind _returnvalue (`PrimitiveComponent.CreateDynamicMaterialInstance` (`self.Balloon`) 0 "/Game/Materials/ColorMaterials/Constants/M_Color_Inst.M_Color_Inst" "None"))
  (`MaterialInstanceDynamic.SetVectorParameterValue` _returnvalue "Color" (`|GetArrayItem` (`/Game/FirstPersonBP/Blueprints/FirstPersonCharacter.WaterBalloonColor` (`self.PlayerRef`))))
  (`PrimitiveComponent.IgnoreActorWhenMoving` (`self.Balloon`) (`GameplayStatics.GetPlayerCharacter` 0) true))

(event `self.ReceiveHit`
  (params (MyComp :type "PrimitiveComponent Object Reference") (Other :type "Actor Object Reference") (OtherComp :type "PrimitiveComponent Object Reference") (bSelfMoved :type Boolean) (HitLocation :type "Vector Structure") (HitNormal :type "Vector Structure") (NormalImpulse :type "Vector Structure") (Hit :type "HitResult Structure (by ref)"))
  (bind _waterburst (`self.WaterBurst`))
  (`ActorComponent.Activate` _waterburst false)
  (`SceneComponent.SetHiddenInGame` (`self.Balloon`) true false)
  (add `NiagaraComponent.OnSystemFinished` _waterburst (delegate `Destroy Actor`)))

(event `Destroy Actor`
  (params (PSystem :type "NiagaraComponent Object Reference"))
  (`/Engine/EditorBlueprintResources/StandardMacros.DoOnce` false
    (:`Completed`
      (`self.Destroy Actor` null))))

(fn `UserConstructionScript`)