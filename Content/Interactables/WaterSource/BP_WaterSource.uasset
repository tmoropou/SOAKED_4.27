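; Interactable water source that refills the water level of the weapon item the player is holding.
; Interaction starts a looping timer that increments the held item's WaterLevel up to its maximum and tells the item to start its water balloon fill.
; Stopping interaction or leaving the interactable area clears the timer and sends the stop-fill message.
; Leaving the area also unregisters the source from the first-person character.
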(event `/Game/Interactables/BPI_Interact.Interaction`
  (params (Instigator :type "/Game/FirstPersonBP/Blueprints/FirstPersonCharacter Object Reference") (Interactable :type "/Game/Interactables/BaseInteractable Object Reference"))
  (bind _itemattached (`/Game/FirstPersonBP/Blueprints/FirstPersonCharacter.ItemAttached` Instigator))
  (`/Engine/EditorBlueprintResources/StandardMacros.IsValid` _itemattached
    (:`Is Valid`
      (switch `/Game/Interactables/E_ItemType` (`/Game/Interactables/BaseInteractable.ItemType` _itemattached)
        (:`NewEnumerator0`
          (`KismetSystemLibrary.K2_SetTimerDelegate` (delegate `StartWaterFlow`) 0.2 true)
          (message `/Game/Interactables/WaterSource/BPI_WaterSource.StartFillWaterBalloon` (`/Game/FirstPersonBP/Blueprints/FirstPersonCharacter.ItemAttached` (`self.PlayerCharRef`))))))))

(event `StartWaterFlow`
  (bind _itemattached (`/Game/FirstPersonBP/Blueprints/FirstPersonCharacter.ItemAttached` (`self.PlayerCharRef`)))
  (`/Engine/EditorBlueprintResources/StandardMacros.IsValid` _itemattached
    (:`Is Valid`
      (if (< (`/Game/Interactables/Soakers/BP_MainWeapon.WaterLevel` _itemattached) (`/Game/Interactables/Soakers/BP_MainWeapon.MaxWaterLevel` _itemattached))
        (`/Engine/EditorBlueprintResources/StandardMacros.IncrementInt` (`/Game/Interactables/Soakers/BP_MainWeapon.WaterLevel` (`/Game/FirstPersonBP/Blueprints/FirstPersonCharacter.ItemAttached` (`self.PlayerCharRef`))))))))

(event `/Game/Interactables/BPI_Interact.StopInteraction`
  (params (Instigator :type "/Game/FirstPersonBP/Blueprints/FirstPersonCharacter Object Reference") (Interactable :type "/Game/Interactables/BaseInteractable Object Reference"))
  (bind _itemattached (`/Game/FirstPersonBP/Blueprints/FirstPersonCharacter.ItemAttached` (`self.PlayerCharRef`)))
  (`KismetSystemLibrary.K2_ClearTimer` null "StartWaterFlow")
  (`/Engine/EditorBlueprintResources/StandardMacros.IsValid` _itemattached
    (:`Is Valid`
      (message `/Game/Interactables/WaterSource/BPI_WaterSource.StopFillWaterBalloon` _itemattached))))

(event `self.Interactable Area.OnComponentEndOverlap`
  (params (OverlappedComponent :type "PrimitiveComponent Object Reference") (OtherActor :type "Actor Object Reference") (OtherComp :type "PrimitiveComponent Object Reference") (OtherBodyIndex :type Integer))
  (bind _playercharref (`self.PlayerCharRef`))
  (bind _itemattached (`/Game/FirstPersonBP/Blueprints/FirstPersonCharacter.ItemAttached` _playercharref))
  (bind _asfirst_person_character (cast `/Game/FirstPersonBP/Blueprints/FirstPersonCharacter` OtherActor))
  (message `/Game/Interactables/BPI_Interact.UnregisterInteractable` _asfirst_person_character self)
  (set `/Game/FirstPersonBP/Blueprints/FirstPersonCharacter.OverlappingActor?` false _playercharref)
  (`KismetSystemLibrary.K2_ClearTimer` null "StartWaterFlow")
  (`/Engine/EditorBlueprintResources/StandardMacros.IsValid` _itemattached
    (:`Is Valid`
      (message `/Game/Interactables/WaterSource/BPI_WaterSource.StopFillWaterBalloon` _itemattached))))

(fn `UserConstructionScript`
  (`parent.UserConstructionScript`))