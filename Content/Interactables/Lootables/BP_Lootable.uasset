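; BP_Lootable is an interactable loot container that opens once and reveals random loot.
; Its Interaction event disables the interact collision, then spawns three random picks from the RandomActorSpawn array, attached at the Loot1–3 points.
; The OpenBin timeline rotates the arrow and raises the bin center, then turns off the mesh's custom-depth rendering.
; An OpenLootContainerRPC event exists but is empty, and its call is unwired.
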(event `/Game/Interactables/BPI_Interact.Interaction`
  (params (Instigator :type "/Game/FirstPersonBP/Blueprints/FirstPersonCharacter Object Reference") (Interactable :type "/Game/Interactables/BaseInteractable Object Reference") (OwningPlayer :type "Actor Object Reference"))
  (if (not (`self.IsBinOpen?`))
    (set `self.IsBinOpen?` true)
    (`PrimitiveComponent.SetCollisionEnabled` (`self.Interactable Area`) "NoCollision")
    (`self.GenerateRandomLoot`)
    (bind (_direction _rotationlerp) (`Timeline|OpenBin`)
      (:`Update`
        (`SceneComponent.K2_SetRelativeRotation` (`self.Arrow`) (`KismetMathLibrary.RLerp` (`self.InitialRotation`) (`self.TargetRotation`) _rotationlerp) false false)
        (`SceneComponent.K2_SetRelativeLocation` (`self.Bin_Center`) (`KismetMathLibrary.VLerp` (0.0 0.0 0.0) (0.0 0.0 30.0) _rotationlerp) false false))
      (:`Finished`
        (`PrimitiveComponent.SetRenderCustomDepth` (`self.Mesh_Stat`) false)))))

(event `OpenLootContainerRPC`)

(fn `GenerateRandomLoot`
  (`|ExecutionSequence`
    (:`then_0`
      (`self.SpawnRandomActor` (`self.Loot1`)))
    (:`then_1`
      (`self.SpawnRandomActor` (`self.Loot2`)))
    (:`then_2`
      (`self.SpawnRandomActor` (`self.Loot3`)))))

(fn `SpawnRandomActor`
  (params (LocationActor :type "SceneComponent Object Reference"))
  (bind _returnvalue (`|SpawnActorFromClass` (`|GetArrayItem` (`self.RandomActorSpawn`) (`KismetMathLibrary.RandomIntegerInRange` 0 (- (`KismetArrayLibrary.Array_Length` (`self.RandomActorSpawn`)) 1))) (`KismetMathLibrary.MakeTransform` (`SceneComponent.K2_GetComponentLocation` LocationActor)) "Undefined" "OverrideRootScale" null null))
  (`self.K2_AttachToComponent` _returnvalue LocationActor "None" "SnapToTarget" "SnapToTarget" "KeepRelative" true))

(fn `UserConstructionScript`
  (`parent.UserConstructionScript`))