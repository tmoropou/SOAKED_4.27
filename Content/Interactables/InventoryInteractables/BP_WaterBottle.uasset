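; Water bottle inventory interactable that the player picks up to gain reserve water.
; On Interaction, it runs PickupItem only if HasSpace passes.
; PickupItem destroys the actor, adds BP_WaterBottle to the player character's ItemInventory and increases ReserveWater by WaterToAdd.
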(event `/Game/Interactables/BPI_Interact.Interaction`
  (params (Instigator :type "/Game/FirstPersonBP/Blueprints/FirstPersonCharacter Object Reference") (Interactable :type "/Game/Interactables/BaseInteractable Object Reference"))
  (if (`self.HasSpace`)
    (`self.PickupItem`)))

(fn `PickupItem`
  (bind _playercharref (`self.PlayerCharRef`))
  (`self.K2_DestroyActor`)
  (`KismetArrayLibrary.Array_Add` (`/Game/FirstPersonBP/Blueprints/FirstPersonCharacter.ItemInventory` (`self.PlayerCharRef`)) "BP_WaterBottle_C")
  (set `/Game/FirstPersonBP/Blueprints/FirstPersonCharacter.ReserveWater` (+ (`/Game/FirstPersonBP/Blueprints/FirstPersonCharacter.ReserveWater` _playercharref) (`self.WaterToAdd`)) _playercharref))

(fn `UserConstructionScript`
  (`parent.UserConstructionScript`))