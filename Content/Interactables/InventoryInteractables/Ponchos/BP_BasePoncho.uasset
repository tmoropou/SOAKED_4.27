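; Base interactable poncho pickup that upgrades the player's wetness protection.
; On interaction, it switches on the currently worn poncho and uses CanEquipPoncho to compare protection against this one's AddedWetnessLevel.
; FindHighlightedPoncho derives a Weak, Average or Strong tier from that level using thresholds.
; PickupPoncho raises the player's MaxWetness, stores the tier and destroys the actor, and the interaction calls CanStartDrying on the player.
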(event `/Game/Interactables/BPI_Interact.Interaction`
  (params (Instigator :type "/Game/FirstPersonBP/Blueprints/FirstPersonCharacter Object Reference") (Interactable :type "/Game/Interactables/BaseInteractable Object Reference"))
  (bind _f_playeritems_poncho (break `/Game/Interactables/InventoryInteractables/F_PlayerItems` (`/Game/FirstPersonBP/Blueprints/FirstPersonCharacter.F_PlayerItems` Instigator)))
  (switch `/Game/Interactables/InventoryInteractables/E_Poncho` _f_playeritems_poncho
    (:`NewEnumerator0`
      (`self.FindHighlightedPoncho`)
      (`self.PickupPoncho`))
    (:`NewEnumerator1`
      (`self.CanEquipPoncho` (`self.WeakPonchoProtection`))
      (`self.FindHighlightedPoncho`)
      (`self.PickupPoncho`))
    (:`NewEnumerator2`
      (`self.CanEquipPoncho` (`self.AveragePonchoProtection`))
      (`self.FindHighlightedPoncho`)
      (`self.PickupPoncho`))
    (:`NewEnumerator3`
      (`self.CanEquipPoncho` (`self.StrongPonchoProtection`))
      (`self.FindHighlightedPoncho`)
      (`self.PickupPoncho`)))
  (`/Game/FirstPersonBP/Blueprints/FirstPersonCharacter.CanStartDrying` (`self.PlayerCharRef`)))

(fn `FindHighlightedPoncho`
  (if (> (`self.AddedWetnessLevel`) 25.0)
    (if (> (`self.AddedWetnessLevel`) 50.0)
      (set `self.HighlightedPoncho` "NewEnumerator3")
      (else
        (set `self.HighlightedPoncho` "NewEnumerator2")))
    (else
      (set `self.HighlightedPoncho` "NewEnumerator1"))))

(fn `PickupPoncho`
  (set `/Game/FirstPersonBP/Blueprints/FirstPersonCharacter.MaxWetness` (+ (`self.AddedWetnessLevel`) 100.0) (`self.PlayerCharRef`))
  (`self.K2_DestroyActor`)
  (set `/Game/FirstPersonBP/Blueprints/FirstPersonCharacter.F_PlayerItems` (make `/Game/Interactables/InventoryInteractables/F_PlayerItems` (`self.HighlightedPoncho`)) (`self.PlayerCharRef`)))

(fn `UserConstructionScript`
  (`parent.UserConstructionScript`))