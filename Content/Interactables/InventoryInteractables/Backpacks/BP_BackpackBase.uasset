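; Base interactable backpack pickup that expands the player's backpack size.
; BeginPlay passes color and spawn rate to its particle system.
; On interaction, only if the instigator has no backpack, it maps its added slot count to a small, medium or large type.
; Pickup adds the slots, destroys the actor, then writes the type and a self reference into the player's items struct, preserving poncho data.
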(event `self.ReceiveBeginPlay`
  (bind _particlesystem (`self.ParticleSystem`))
  (`parent.ReceiveBeginPlay`)
  (`NiagaraComponent.SetVariableLinearColor` _particlesystem "Color" (`self.ParticleColor`))
  (`NiagaraComponent.SetVariableFloat` _particlesystem "SpawnRate" (`self.SpawnRate`)))

(event `/Game/Interactables/BPI_Interact.Interaction`
  (params (Instigator :type "/Game/FirstPersonBP/Blueprints/FirstPersonCharacter Object Reference") (Interactable :type "/Game/Interactables/BaseInteractable Object Reference") (OwningPlayer :type "Actor Object Reference"))
  (bind (_f_playeritems_poncho _f_playeritems_ponchoref _f_playeritems_backpack) (break `/Game/Interactables/InventoryInteractables/F_PlayerItems` (`/Game/FirstPersonBP/Blueprints/FirstPersonCharacter.F_PlayerItems` Instigator)))
  (switch `/Game/Interactables/InventoryInteractables/Backpacks/E_Backpack` _f_playeritems_backpack
    (:`NewEnumerator3`
      (`self.FindHighlightedBackpack`)
      (`self.PickupBackpack`))))

(fn `FindHighlightedBackpack`
  (switch `int` (`self.AddedSlots`)
    (:`2`
      (set `self.HighlightedBackpack` "NewEnumerator0"))
    (:`4`
      (set `self.HighlightedBackpack` "NewEnumerator1"))
    (:`6`
      (set `self.HighlightedBackpack` "NewEnumerator2"))))

(fn `PickupBackpack`
  (bind _playercharref (`self.PlayerCharRef`))
  (bind _playercharref_2 (`self.PlayerCharRef`))
  (bind (_f_playeritems_poncho _f_playeritems_ponchoref) (break `/Game/Interactables/InventoryInteractables/F_PlayerItems` (`/Game/FirstPersonBP/Blueprints/FirstPersonCharacter.F_PlayerItems` _playercharref_2)))
  (set `/Game/FirstPersonBP/Blueprints/FirstPersonCharacter.BackpackSize` (+ (`/Game/FirstPersonBP/Blueprints/FirstPersonCharacter.BackpackSize` _playercharref) (`self.AddedSlots`)) _playercharref)
  (`self.K2_DestroyActor`)
  (set `/Game/FirstPersonBP/Blueprints/FirstPersonCharacter.F_PlayerItems` (make `/Game/Interactables/InventoryInteractables/F_PlayerItems` _f_playeritems_poncho _f_playeritems_ponchoref (`self.HighlightedBackpack`) self) _playercharref_2))

(fn `UserConstructionScript`
  (`parent.UserConstructionScript`))